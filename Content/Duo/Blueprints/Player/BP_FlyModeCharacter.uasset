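; Player character for fly mode that serves as a capture tool for exporting six square directional views (front, right, back, left, top, bottom) from its position.
; O turns the control rotation to each face, running a screenshot console command built from ImageSize, with delays between shots.
; P saves one named screenshot; V, B and N switch window resolution.
; An alternative SceneCapture2D render-target export to a hardcoded folder exists but is never called here.
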(event EventBeginPlay
  (Variables|Default|SetplayerController (Game|GetPlayerController 0)))

(event Input|KeyboardEvents|P
  (params (Key :type Key%20Structure :default "None"))
  (:Pressed
    (Class|FlyModeCharacter|SaveScreenShot (Utilities|String|Append (Variables|Default|GetName) (Variables|Default|GetSuffix)))))

(event Input|KeyboardEvents|N
  (params (Key :type Key%20Structure :default "None"))
  (:Pressed
    (Development|ExecuteConsoleCommand "r.setRes 4096x4096w" 0)))

(event Input|KeyboardEvents|O
  (params (Key :type Key%20Structure :default "None"))
  (:Pressed
    ;[1 1 1] front
    (Pawn|SetControlRotation (Variables|Default|GetplayerController) (Math|Rotator|MakeRotator 0.0 0.0 0.0))
    (CallFunction|ExportScreenShot)
    (Utilities|FlowControl|Delay (Variables|Default|GetwaitTime))
    ;[1 1 1] right
    (Pawn|SetControlRotation (Variables|Default|GetplayerController) (Math|Rotator|MakeRotator 0.0 0.0 -9e+01))
    (CallFunction|ExportScreenShot)
    (Utilities|FlowControl|Delay (Variables|Default|GetwaitTime))
    ;[1 1 1] back
    (Pawn|SetControlRotation (Variables|Default|GetplayerController) (Math|Rotator|MakeRotator 0.0 0.0 1.8e+02))
    (CallFunction|ExportScreenShot)
    (Utilities|FlowControl|Delay (Variables|Default|GetwaitTime))
    ;[1 1 1] left
    (Pawn|SetControlRotation (Variables|Default|GetplayerController) (Math|Rotator|MakeRotator 0.0 0.0 9e+01))
    (CallFunction|ExportScreenShot)
    (Utilities|FlowControl|Delay (Variables|Default|GetwaitTime))
    ;[1 1 1] top
    (Pawn|SetControlRotation (Variables|Default|GetplayerController) (Math|Rotator|MakeRotator 0.0 9e+01 0.0))
    (CallFunction|ExportScreenShot)
    (Utilities|FlowControl|Delay (Variables|Default|GetwaitTime))
    ;[1 1 1] bottom
    (Pawn|SetControlRotation (Variables|Default|GetplayerController) (Math|Rotator|MakeRotator 0.0 -9e+01 0.0))
    (CallFunction|ExportScreenShot)))

(event Input|KeyboardEvents|V
  (params (Key :type Key%20Structure :default "None"))
  (:Pressed
    (Development|ExecuteConsoleCommand "r.setRes 1280x720w" 0)))

(event Input|KeyboardEvents|M
  (params (Key :type Key%20Structure :default "None")))

(event Input|KeyboardEvents|B
  (params (Key :type Key%20Structure :default "None"))
  (:Pressed
    (Development|ExecuteConsoleCommand "r.setRes 2048x2048w" 0)))

(fn ConstructionScript)

(fn ExportImg
  (params (Name :type String) (Target :type Texture%20Render%20Target%202D%20Object%20Reference%20%28by%20ref%29))
  (Utilities|IsValid Target
    (:Is%20Valid
      (Rendering|SceneCapture|CaptureScene (Variables|Default|GetSceneCaptureComponent2D) :!class /Script/Engine.SceneCaptureComponent2D)
      (Rendering|ExportRenderTarget (Variables|Default|GetdefaultTarget2D) "C:\\Hjf\\Study\\UE5\\5.0\\Duo\\Output\\" Name))))

(fn ResetRotation
  (Transformation|SetRelativeRotation (Variables|Default|GetSceneCaptureComponent2D) (Variables|Default|GetOriginalRotator) false false))

(fn Export
  (Variables|Default|SetOriginalRotator (Variables|/Script/Engine.SceneComponent|GetRelativeRotation (Variables|Default|GetSceneCaptureComponent2D)))
  (Transformation|SetRelativeRotation (Variables|Default|GetSceneCaptureComponent2D) "0, 0, 0" false false)
  (CallFunction|ExportImg "front.png" (Variables|Default|GetdefaultTarget2D))
  (Transformation|SetRelativeRotation (Variables|Default|GetSceneCaptureComponent2D) "0,-90.000000, 0" false false)
  (CallFunction|ExportImg "right.png" (Variables|Default|GetdefaultTarget2D))
  (Transformation|SetRelativeRotation (Variables|Default|GetSceneCaptureComponent2D) "0,180.000000, 0" false false)
  (CallFunction|ExportImg "back.png" (Variables|Default|GetdefaultTarget2D))
  (Transformation|SetRelativeRotation (Variables|Default|GetSceneCaptureComponent2D) "0,90.000000, 0" false false)
  (CallFunction|ExportImg "left.png" (Variables|Default|GetdefaultTarget2D))
  (Transformation|SetRelativeRotation (Variables|Default|GetSceneCaptureComponent2D) "90.000000,0.000000,0.000000" false false)
  (CallFunction|ExportImg "top.png" (Variables|Default|GetdefaultTarget2D))
  (Transformation|SetRelativeRotation (Variables|Default|GetSceneCaptureComponent2D) "-90.000000,0.000000,0.000000" false false)
  (CallFunction|ExportImg "bottom.png" (Variables|Default|GetdefaultTarget2D))
  (CallFunction|ResetRotation))

(fn ExportScreenShot
  (bind _command (CallFunction|SpawnCommandStr (Variables|Default|GetImage%20Size)))
  (Development|ExecuteConsoleCommand _command 0))

(fn SpawnCommandStr
  (params (ImageSize :type Integer))
  (bind _returnvalue (Utilities|String|ToString(Integer) ImageSize))
  (LocalVariables|SetImageSizeStr _returnvalue)
  (return (Utilities|String|Append (Variables|Default|GetPrefixCommand) (Utilities|String|Append (Utilities|String|Append _returnvalue "x") (LocalVariables|GetImageSizeStr)))))