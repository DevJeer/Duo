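; BP_Measure is a mouse-driven measuring tool actor, toggled on and off with number keys, that shows distances between points in the world.
; While active, a per-tick cursor line trace moves a marker to the hit point.
; Left click spawns a cable and widget component there; the cable end follows the cursor while WBP_Measure shows meters at the midpoint.
; Right click or disabling removes only the most recent cable and label.
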(event Custom|EnableMeasure
  ;[1 1 1] Enable Measure Function
  (Variables|Default|SetIsMeasuring true)
  (Rendering|SetVisibility (Variables|Default|GetMeasurePoint) true false))

(event Custom|DisableMeasure
  (bind _cableline (Variables|Default|GetCableLine))
  (bind _measureui (Variables|Default|GetMeasureUI))
  ;[1 1 1] Disable Measure Function
  (Variables|Default|SetIsMeasuring false)
  (Rendering|SetVisibility (Variables|Default|GetMeasurePoint) false false)
  (Utilities|FlowControl|Sequence
    (:then_0
      (Utilities|IsValid _cableline
        (:Is%20Valid
          (Components|DestroyComponent _cableline))))
    (:then_1
      (Utilities|IsValid _measureui
        (:Is%20Valid
          (Components|DestroyComponent _measureui))))))

(event Custom|Update
  (bind _returnvalue (Game|GetPlayerController 0))
  (bind _cableline (Variables|Default|GetCableLine))
  (bind (_worldlocation _worlddirection) (Game|Player|ConvertMouseLocationToWorldSpace _returnvalue))
  ;[1 1 1] Line Trace
  (if (Variables|Default|GetIsMeasuring)
    (bind (_outhit _returnvalue_2) (Collision|LineTraceByChannel _worldlocation (+ _worldlocation (* (Variables|Default|GetRayLength) _worlddirection)) "TraceTypeQuery1" true 0 "None"))
    (if _returnvalue_2
      (bind _output_get (Variables|Default|SetHitLocation (.Location (Collision|BreakHitResult _outhit))))
      ;[1 1 1] Update Measure Point
      (Transformation|SetWorldLocation (Variables|Default|GetMeasurePoint) _output_get false false)
      (Utilities|IsValid _cableline
        (:Is%20Valid
          ;[1 1 1] Update Line
          (Variables|/Script/CableComponent.CableComponent|SetEndLocation _cableline (Math|Transform|InverseTransformLocation (Transformation|GetActorTransform) (Variables|Default|GetHitLocation)))
          ;[1 1 1] Update UI Location
          (Transformation|SetWorldLocation (Variables|Default|GetMeasureUI) (/ (+ (Variables|Default|GetHitLocation) (Variables|Default|GetLastClickLocation)) "2.000000,2.000000,2.000000") false false)
          (bind _aswbp_measure (Utilities|Casting|CastToWBP_Measure (UserInterface|GetWidget (Variables|Default|GetMeasureUI))))
          ;[1 1 1] Update UI Text
          (Default|UpdateDistance _aswbp_measure (/ (Math|Vector|Distance(Vector) (Variables|Default|GetHitLocation) (Variables|Default|GetLastClickLocation)) 1e+02)))))))

(event Custom|SpawnLine
  ;[1 1 1] Spawn Line Imp
  (bind _returnvalue (AddComponent|AddCableComponent false (Math|Transform|MakeTransform (Math|Transform|InverseTransformLocation (Transformation|GetActorTransform) (Variables|Default|GetHitLocation)) "0, 0, 0" "0.200000,0.200000,0.200000")))
  (Variables|Default|SetCableLine _returnvalue)
  (Variables|Default|SetLastClickLocation (Variables|Default|GetHitLocation)))

(event Custom|SpawnUI
  ;[1 1 1] Spawn UI Imp
  (bind _returnvalue (AddComponent|AddWidgetComponent false (Math|Transform|MakeTransform (Math|Transform|InverseTransformLocation (Transformation|GetActorTransform) (Variables|Default|GetHitLocation)) "0, 0, 0" "0.500000,0.500000,0.500000")))
  (Variables|Default|SetMeasureUI _returnvalue))

(event EventTick
  (params (DeltaSeconds :type Float%20%28single-precision%29))
  ;[1 1 1] Update
  (CallFunction|Update))

(event EventBeginPlay
  ;[1 1 1] Begin Play
  (Rendering|SetVisibility (Variables|Default|GetMeasurePoint) false false))

(event Input|KeyboardEvents|1
  (params (Key :type Key%20Structure :default "None"))
  ;[1 1 1] Enable Measure Trigger
  (:Pressed
    (CallFunction|EnableMeasure)))

(event Input|KeyboardEvents|2
  (params (Key :type Key%20Structure :default "None"))
  ;[1 1 1] Disable Measure Trigger
  (:Pressed
    (CallFunction|DisableMeasure)))

(event Input|MouseEvents|LeftMouseButton
  (params (Key :type Key%20Structure :default "None"))
  ;[1 1 1] Spawn Line and UI Trigger
  (:Pressed
    (if (Variables|Default|GetIsMeasuring)
      (CallFunction|SpawnLine)
      (CallFunction|SpawnUI))))

(event Input|MouseEvents|RightMouseButton
  (params (Key :type Key%20Structure :default "None"))
  (bind _cableline (Variables|Default|GetCableLine))
  (bind _measureui (Variables|Default|GetMeasureUI))
  ;[1 1 1] Break Line and UI
  (:Pressed
    (if (Variables|Default|GetIsMeasuring)
      (Utilities|FlowControl|Sequence
        (:then_0
          (Utilities|IsValid _cableline
            (:Is%20Valid
              (Components|DestroyComponent _cableline))))
        (:then_1
          (Utilities|IsValid _measureui
            (:Is%20Valid
              (Components|DestroyComponent _measureui))))))))

(fn ConstructionScript)