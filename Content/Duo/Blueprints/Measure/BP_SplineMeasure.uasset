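; Mouse-driven distance measuring tool actor, switched on and off with keys 1 and 2.
; While active, Tick traces under the cursor to move a marker icon to the hit point.
; Left click spawns a spline, spline mesh line and widget; Tick stretches the newest line to the cursor, showing metres at its midpoint via WBP_Measure.
; Right click or disabling destroys only the latest set, as earlier references are overwritten.
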(event Custom|EnableMeasure
  ;[1 1 1] Enable Measure Imp
  (Rendering|SetVisibility (Variables|Default|GetMeasureIcon) true false)
  (Variables|Default|SetIsTracing true)
  (Variables|/Script/Engine.PlayerController|SetbShowMouseCursor (Game|GetPlayerController 0) false))

(event Custom|DisableMeasure
  ;[1 1 1] Disable Measure Imp
  (Rendering|SetVisibility (Variables|Default|GetMeasureIcon) false false)
  (Variables|Default|SetIsTracing false)
  (Variables|/Script/Engine.PlayerController|SetbShowMouseCursor (Game|GetPlayerController 0) true)
  (CallFunction|CleanLineandText))

(event Custom|Update
  (bind _returnvalue (Game|GetPlayerController 0))
  (bind _spline (Variables|Default|GetSpline))
  (bind _spline_2 (Variables|Default|GetSpline))
  (bind _spline_3 (Variables|Default|GetSpline))
  (bind _wbp_measure (Variables|Default|GetWBP_Measure))
  (bind (_worldlocation _worlddirection) (Game|Player|ConvertMouseLocationToWorldSpace _returnvalue))
  (bind (_location _tangent) (Spline|GetLocationandTangentatSplinePoint _spline_2 1 "World"))
  (bind (_location_2 _tangent_2) (Spline|GetLocationandTangentatSplinePoint _spline_3 0 "World"))
  ;[1 1 1] Update
  (if (Variables|Default|GetIsTracing)
    ;;[1 1 1] Line Track at mouse click position
    (bind (_outhit _returnvalue_2) (Collision|LineTraceByChannel _worldlocation (+ _worldlocation (* _worlddirection "10000.000000,10000.000000,10000.000000")) "TraceTypeQuery1" true 0 "None"))
    (if _returnvalue_2
      ;;[1 1 1] Set Measure Icon Location
      (Variables|Default|SetMouseHitLocation (.Location (Collision|BreakHitResult _outhit)))
      (Transformation|SetWorldLocation (Variables|Default|GetMeasureIcon) (Variables|Default|GetMouseHitLocation) false false)
      (Utilities|IsValid _spline
        (:Is%20Valid
          ;;[1 1 1] Set Point Of Spline Component
          (Spline|SetLocationatSplinePoint _spline 1 (Variables|Default|GetMouseHitLocation) "World" true)
          (Utilities|IsValid (Variables|Default|GetSplineMesh)
            (:Is%20Valid
              ;;[1 1 1] Set Spline Mesh Location And Tangent
              (SplineMesh|SetStartandEnd (Variables|Default|GetSplineMesh) _location_2 _tangent_2 _location _tangent true :!class /Script/Engine.SplineMeshComponent)
              (Utilities|IsValid _wbp_measure
                (:Is%20Valid
                  ;;[1 1 1] Set Distance Text Location
                  (Transformation|SetWorldLocation _wbp_measure (/ (+ (Variables|Default|GetLastMouseHitLocation) (Variables|Default|GetMouseHitLocation)) "2.000000,2.000000,2.000000") false false)
                  (bind _aswbp_measure (Utilities|Casting|CastToWBP_Measure (UserInterface|GetWidget (Variables|Default|GetWBP_Measure))))
                  ;;[1 1 1] Update Distance Text
                  (Default|UpdateDistance _aswbp_measure (/ (Math|Vector|Distance(Vector) (Variables|Default|GetLastMouseHitLocation) (Variables|Default|GetMouseHitLocation)) 1e+02)))))))))))

(event EventBeginPlay
  (bind _returnvalue (Game|GetPlayerController 0))
  ;[1 1 1] BeginPlay
  (Input|SetInputModeGameandUI _returnvalue 0 "DoNotLock" true)
  (Input|EnableInput _returnvalue)
  (Rendering|SetVisibility (Variables|Default|GetMeasureIcon) false false))

(event EventTick
  (params (DeltaSeconds :type Float%20%28single-precision%29))
  ;[1 1 1] Tick
  (CallFunction|Update))

(event Input|KeyboardEvents|1
  (params (Key :type Key%20Structure :default "None"))
  ;[1 1 1] Enable Measure
  (:Pressed
    (CallFunction|EnableMeasure)))

(event Input|KeyboardEvents|2
  (params (Key :type Key%20Structure :default "None"))
  ;[1 1 1] Disable Measure
  (:Pressed
    (CallFunction|DisableMeasure)))

(event Input|MouseEvents|LeftMouseButton
  (params (Key :type Key%20Structure :default "None"))
  ;[1 1 1] Left Mouse Button Click
  (:Pressed
    (if (Variables|Default|GetIsTracing)
      (CallFunction|SpawnSpline)
      (Variables|Default|SetLastMouseHitLocation (Variables|Default|GetMouseHitLocation))
      (CallFunction|SpawnUI))))

(event Input|MouseEvents|RightMouseButton
  (params (Key :type Key%20Structure :default "None"))
  ;[1 1 1] Right Mouse Button Click
  (:Pressed
    (if (Variables|Default|GetIsTracing)
      (CallFunction|CleanLineandText))))

(fn ConstructionScript)

(fn SpawnSpline
  (bind _returnvalue (Transformation|GetActorTransform))
  (bind _mousehitlocation (Variables|Default|GetMouseHitLocation))
  (bind _linescale (Variables|LineConfig|GetLineScale))
  ;[1 1 1] Create Spline Component
  (bind _returnvalue_2 (AddComponent|AddSplineComponent false (Math|Transform|MakeTransform (Math|Transform|InverseTransformLocation _returnvalue _mousehitlocation) (Math|Conversions|RotationFromXVector (Math|Transform|InverseTransformDirection _returnvalue _mousehitlocation)))))
  (Variables|Default|SetSpline _returnvalue_2)
  ;[1 1 1] Create Spline Mesh Component
  (bind _returnvalue_3 (AddComponent|AddSplineMeshComponent true (Math|Transform|MakeTransform (.Location (Spline|GetLocationandTangentatSplinePoint (Variables|Default|GetSpline) 0 "Local")) (Math|Conversions|RotationFromXVector (.Tangent (Spline|GetLocationandTangentatSplinePoint (Variables|Default|GetSpline) 0 "Local"))))))
  (Variables|Default|SetSplineMesh _returnvalue_3)
  (Rendering|Material|SetMaterial (Variables|Default|GetSplineMesh) 0 (Variables|LineConfig|GetLineMaterial))
  (SplineMesh|SetStartScale (Variables|Default|GetSplineMesh) _linescale true :!class /Script/Engine.SplineMeshComponent)
  (SplineMesh|SetEndScale (Variables|Default|GetSplineMesh) _linescale true :!class /Script/Engine.SplineMeshComponent))

(fn SpawnUI
  ;[1 1 1] Create Mesaure Text
  (bind _returnvalue (AddComponent|AddWidgetComponent false (Math|Transform|MakeTransform (Math|Transform|InverseTransformDirection (Transformation|GetActorTransform) (Variables|Default|GetMouseHitLocation)))))
  (Variables|Default|SetWBP_Measure _returnvalue))

(fn CleanLineandText
  (bind _splinemesh (Variables|Default|GetSplineMesh))
  (bind _spline (Variables|Default|GetSpline))
  (bind _wbp_measure (Variables|Default|GetWBP_Measure))
  (Utilities|IsValid _splinemesh
    (:Is%20Valid
      ;[1 1 1] Destroy Spline Mesh Comp
      (Components|DestroyComponent _splinemesh)
      (Utilities|IsValid _spline
        (:Is%20Valid
          ;[1 1 1] Destroy Spline Component
          (Components|DestroyComponent _spline)
          (Utilities|IsValid _wbp_measure
            (:Is%20Valid
              ;[1 1 1] Destroy Measure Text
              (Components|DestroyComponent _wbp_measure))))))))